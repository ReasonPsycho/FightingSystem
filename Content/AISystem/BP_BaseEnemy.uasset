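; BP_BaseEnemy is a base enemy Blueprint that provides a melee attack against a given target actor.
; Its Attack event, skipped while the HealthComponent reports dying, runs a multi sphere trace for pawns around the enemy, with debug drawing on.
; If the target is among the hits, it applies fixed damage, plays an attack montage and stops checking further hits.
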(event EventBeginPlay)

(event EventAttack
  (params (TargetActor :type Actor%20Object%20Reference))
  (bind _returnvalue (Transformation|GetActorLocation))
  (if (not (Class|HealthComponent|Dying (Variables|Default|GetHealthComponent)))
    (bind (_outhits _returnvalue_2) (Collision|MultiSphereTraceForObjects _returnvalue _returnvalue 2e+02 (Utilities|Array|MakeArray "ObjectTypeQuery3") false 0 "ForDuration"))
    (if _returnvalue_2
      (bind _array_element (Utilities|Array|ForEachLoopwithBreak _outhits :!label _label)
        (:LoopBody
          (if (== (.HitActor (Collision|BreakHitResult _array_element)) TargetActor)
            (Game|Damage|ApplyDamage (.HitActor (Collision|BreakHitResult _array_element)) 1e+01 0 0)
            (Animation|Montage|PlayMontage (Variables|Character|GetMesh) "/Game/Characters/Mannequins/Anims/Unarmed/Attack/MM_Attack_01_Montage.MM_Attack_01_Montage"
              (:then
                (goto _label Break)))))))))

(fn ConstructionScript)