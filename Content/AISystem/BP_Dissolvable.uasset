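; BP_Dissolvable is an actor that plays a dissolve effect when something overlaps its Sphere1 component, then destroys itself.
; On BeginPlay it creates a dynamic instance of M_Dissolve and applies it to the Sphere component.
; Dissolve sets a threshold, then a timeline drives the material's dissolve, squash, deform and levitation parameters before the actor is destroyed.
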(event OnComponentBeginOverlap(Sphere1)
  (params (OverlappedComponent :type Primitive%20Component%20Object%20Reference) (OtherActor :type Actor%20Object%20Reference) (OtherComp :type Primitive%20Component%20Object%20Reference) (OtherBodyIndex :type Integer) (bFromSweep :type Boolean) (SweepResult :type Hit%20Result%20Structure%20%28by%20ref%29))
  (CallFunction|Dissolve))

(event Custom|Dissolve
  (bind _materialref (Variables|Default|GetMaterialRef))
  (Rendering|Material|SetScalarParameterValue (Variables|Default|GetMaterialRef) "Treshold" 0.2 :!class /Script/Engine.MaterialInstanceDynamic)
  (bind (_direction _dissolve_track _squash_track _deform_track _levitation_track) (Timeline|DissolveTimeline Play)
    (:Update
      (Rendering|Material|SetScalarParameterValue _materialref "Dissolve" _dissolve_track :!class /Script/Engine.MaterialInstanceDynamic)
      (Rendering|Material|SetScalarParameterValue _materialref "SquashTime" _squash_track :!class /Script/Engine.MaterialInstanceDynamic)
      (Rendering|Material|SetScalarParameterValue _materialref "DeformStrength" _deform_track :!class /Script/Engine.MaterialInstanceDynamic)
      (Rendering|Material|SetScalarParameterValue _materialref "Levitation" _levitation_track :!class /Script/Engine.MaterialInstanceDynamic))
    (:Finished
      (Actor|DestroyActor))))

(event EventBeginPlay
  (bind _returnvalue (Rendering|Material|CreateDynamicMaterialInstance "/Game/Materials/M_Dissolve.M_Dissolve" "None" "None" :!class /Script/Engine.KismetMaterialLibrary))
  (bind _output_get (Variables|Default|SetMaterialRef _returnvalue))
  (Rendering|Material|SetMaterial (Variables|Default|GetSphere) 0 _output_get))

(fn ConstructionScript)