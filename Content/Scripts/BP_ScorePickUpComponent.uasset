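; Spawner actor that scatters ScorePickUp actors across a random subset of its eight calibration points when play begins.
; BeginPlay shuffles the points, then spawns pickups at the leading entries up to a random index, so both layout and count vary while each point is used at most once.
; AllScores increments with every spawn to track the total, and the overlap and Tick events do nothing.
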(event EventBeginPlay
  (bind _output_get (Variables|Default|SetSpawnPointsArray (Utilities|Array|MakeArray (Variables|Default|GetCalibrationPoint) (Variables|Default|GetCalibrationPoint1) (Variables|Default|GetCalibrationPoint2) (Variables|Default|GetCalibrationPoint3) (Variables|Default|GetCalibrationPoint4) (Variables|Default|GetCalibrationPoint5) (Variables|Default|GetCalibrationPoint6) (Variables|Default|GetCalibrationPoint7))))
  (Utilities|Array|Shuffle _output_get)
  (for _index (range 0 (Math|Random|RandomIntegerinRange 5 (Utilities|Array|LastIndex _output_get)))
    (Game|SpawnActorfromClass "/Game/TopDown/Blueprints/Buffs/ScorePickUp.ScorePickUp_C" (Transformation|GetWorldTransform (Utilities|Array|Get(acopy) _output_get _index)) "AdjustIfPossibleButAlwaysSpawn" "MultiplyWithRoot" 0 0)
    (bind _result (Math|Integer|IncrementInt (Variables|Default|GetAllScores))
      (:%20%20
        (Variables|Default|SetAllScores _result)))))

(event Collision|EventActorBeginOverlap
  (params (OtherActor :type Actor%20Object%20Reference)))

(event EventTick
  (params (DeltaSeconds :type Float%20%28single-precision%29)))

(fn ConstructionScript)