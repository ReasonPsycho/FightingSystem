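; BP_ScorePickup is a one-shot trigger that spawns score pickups when a BP_TopDownCharacter overlaps it.
; The overlap sets a HasSpawned flag and calls SpawnScorePickUp, which also has a DoOnce before its loop.
; The loop, bounded by SpawnCount, spawns the ScorePickUp class at the actor's location offset by SpawnPoint, copying its rotation and scale.
; All spawns share that point, adjusted for collisions where possible.
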(event EventBeginPlay)

(event Collision|EventActorBeginOverlap
  (params (OtherActor :type Actor%20Object%20Reference))
  (Utilities|Casting|CastToBP_TopDownCharacter OtherActor)
  (if (not (Variables|Default|GetbHasSpawned))
    (Variables|Default|SetbHasSpawned true)
    (CallFunction|SpawnScorePickUp)))

(event EventTick
  (params (DeltaSeconds :type Float%20%28single-precision%29)))

(fn ConstructionScript)

(fn SpawnScorePickUp
  (bind _returnvalue (Transformation|GetActorTransform))
  (bind (_location _rotation _scale) (Math|Transform|BreakTransform _returnvalue))
  (Utilities|FlowControl|DoOnce false
    (:Completed
      (for _index (range 0 (Variables|Default|GetspawnCount))
        (Game|SpawnActorfromClass "/Game/TopDown/Blueprints/Buffs/ScorePickUp.ScorePickUp_C" (Math|Transform|MakeTransform (+ _location (.Location (Math|Transform|BreakTransform (Variables|Default|GetspawnPoint)))) _rotation _scale) "AdjustIfPossibleButAlwaysSpawn" "MultiplyWithRoot" 0 0)))))